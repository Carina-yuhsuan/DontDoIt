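; SpikeWallBP is a Stage 3 spike-wall trap that drops once and kills the player on contact.
; Its Fall function, not called within this Blueprint, enables physics on the Plane and plays a chain sound, guarded by the Actived flag to fire only once.
; Box overlap with a BP_Player runs its DeathProcess, then reloads the current level by name after a short delay.
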(event `self.Box.OnComponentBeginOverlap`
  (params (OverlappedComponent :type "PrimitiveComponent Object Reference") (OtherActor :type "Actor Object Reference") (OtherComp :type "PrimitiveComponent Object Reference") (OtherBodyIndex :type Integer) (bFromSweep :type Boolean) (SweepResult :type "HitResult Structure (by ref)"))
  (bind _asbp_player (cast `/Game/OuKanu/Character/BP_Player` OtherActor))
  (`/Engine/EditorBlueprintResources/StandardMacros.IsValid` _asbp_player
    (:`Is Valid`
      (`/Game/OuKanu/Character/BP_Character.DeathProcess` _asbp_player)
      (`KismetSystemLibrary.Delay` 3.0)
      (bind _returnvalue (`GameplayStatics.GetCurrentLevelName` true))
      (`GameplayStatics.OpenLevel` (`KismetStringLibrary.Conv_StringToName` _returnvalue)))))

(fn `fall`
  (if (not (`self.actived`))
    (`PrimitiveComponent.SetSimulatePhysics` (`self.Plane`) true)
    (`GameplayStatics.PlaySoundAtLocation` "/Game/Duarte/DuarteResources/UI/ChainEffect.ChainEffect" (`SceneComponent.RelativeLocation` (`self.Plane`)) (struct) 1.0 1.0 0.0 null null null)
    (set `self.actived` true)))

(fn `UserConstructionScript`)