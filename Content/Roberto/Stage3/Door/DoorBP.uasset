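; DoorBP is a level exit door that sends the player to the next level once it has been opened.
; The OpenDoor event blacks out the closed door's material, reveals the open door component and sets an Open flag.
; When BP_Player overlaps the Box trigger while Open is set, it loads the level named by the Nextlevel variable.
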(event `OpenDoor`
  (`PrimitiveComponent.SetMaterial` (`self.DoorClosed`) 0 "/Game/Duarte/DuarteResources/DuarteMaterials/Black.Black")
  (`SceneComponent.SetVisibility` (`self.DoorOpen`) true false)
  (set `self.open` true))

(event `self.Box.OnComponentBeginOverlap`
  (params (OverlappedComponent :type "PrimitiveComponent Object Reference") (OtherActor :type "Actor Object Reference") (OtherComp :type "PrimitiveComponent Object Reference") (OtherBodyIndex :type Integer) (bFromSweep :type Boolean) (SweepResult :type "HitResult Structure (by ref)"))
  (bind _asbp_player (cast `/Game/OuKanu/Character/BP_Player` OtherActor))
  (`/Engine/EditorBlueprintResources/StandardMacros.IsValid` _asbp_player
    (:`Is Valid`
      (if (`self.open`)
        (`GameplayStatics.OpenLevel` (`KismetStringLibrary.Conv_StringToName` (`self.nextlevel`)))))))

(fn `UserConstructionScript`)