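; BossRockBP is a rock projectile, apparently for a boss enemy, that damages the player on contact.
; INITIALIZE gives the Model a random non-uniform scale and resets the actor's relative location to zero.
; MoveRock moves the Model to a supplied relative position over one second.
; On overlap with BP_Player, it plays a hurt sound, sends HurtMessage, spawns a hit emitter and destroys itself.
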(event `MoveRock`
  (params (ActorPos :type "Vector Structure"))
  (`KismetSystemLibrary.MoveComponentTo` (`self.Model`) ActorPos (struct) false false 1.0))

(event `self.ReceiveTick`
  (params (DeltaSeconds :type "Float (single-precision)")))

(event `INITIALIZE`
  (`self.SetSize`)
  (`self.SetLocation`))

(event `self.Model.OnComponentBeginOverlap`
  (params (OverlappedComponent :type "PrimitiveComponent Object Reference") (OtherActor :type "Actor Object Reference") (OtherComp :type "PrimitiveComponent Object Reference") (OtherBodyIndex :type Integer) (bFromSweep :type Boolean) (SweepResult :type "HitResult Structure (by ref)"))
  (bind (_returnvalue_location _returnvalue_rotation _returnvalue_scale) (`KismetMathLibrary.BreakTransform` (`self.GetTransform`)))
  (bind _relativelocation (`SceneComponent.RelativeLocation` (`self.Model`)))
  (bind _asbp_player (cast `/Game/OuKanu/Character/BP_Player` OtherActor))
  (`/Engine/EditorBlueprintResources/StandardMacros.IsValid` _asbp_player
    (:`Is Valid`
      (`GameplayStatics.PlaySoundAtLocation` "/Game/Roberto/AudioManager/Music/SFX_Cue/Player_Hurt.Player_Hurt" _relativelocation (struct) 1.0 1.0 0.0 null null null)
      (message `/Game/OuKanu/BP/Interface/BPI_Character.Hurt` _asbp_player 10.0)
      (`GameplayStatics.SpawnEmitterAtLocation` "/Game/OuKanu/FX/FXVarietyPack/Particles/P_ky_hit2.P_ky_hit2" _relativelocation _returnvalue_rotation _returnvalue_scale)
      (`self.K2_DestroyActor`))))

(fn `SetLocation`
  (`self.K2_SetActorRelativeLocation` (0.0 0.0 0.0)))

(fn `SetSize`
  (set `self.x` (`KismetMathLibrary.RandomFloatInRange` 0.1 1.0))
  (set `self.y` (`KismetMathLibrary.RandomFloatInRange` 0.1 1.0))
  (set `self.z` (`KismetMathLibrary.RandomFloatInRange` 0.1 1.0))
  (`SceneComponent.SetRelativeScale3D` (`self.Model`) (`KismetMathLibrary.MakeVector` (`self.x`) (`self.y`) (`self.z`))))

(fn `UserConstructionScript`)